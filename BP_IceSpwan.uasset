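; BP_IceSpwan is a spawner that drops ice hazards at random spots within its UnderBox bounds.
; A looping timer started on BeginPlay randomly picks a short delay or a longer one before each spawn.
; Both paths, one inline and one through IceSpawn, place a red BP_Ice_Point marker, then spawn BP_Ice high above it a second later.
; Older loop-based spawn chains remain in the graph unconnected.
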(event Custom|Spawn_Ice%201
  (bind _under_box (Variables|Default|GetUnder_Box))
  ;[1 0.43 0.6021] とりあえずDelayでランダムに
  (if (Math|Random|RandomBool)
    (Utilities|FlowControl|Delay 1.0)
    (bind _returnvalue (Game|SpawnActorfromClass "/Game/IceCatch/BP_Ice_Point.BP_Ice_Point_C" (Math|Transform|MakeTransform (- (Math|Random|RandomPointinBoundingBox (Transformation|GetWorldLocation _under_box) (Variables|/Script/Engine.BoxComponent|GetBoxExtent _under_box)) "") "0, 0, 0" "1.000000,1.000000,1.000000") "Undefined" 0 0)) ; 先ず赤ポイントをスポーン
    (Utilities|FlowControl|Delay 1.0)
    (Game|SpawnActorfromClass "/Game/IceCatch/BP_Ice.BP_Ice_C" (Math|Transform|MakeTransform (+ (.location (Transformation|GetActorTransform _returnvalue)) "0,0,1000.000000") "0, 0, 0" "1.000000,1.000000,1.000000") "Undefined" 0 0) ; スポーンする
    (else
      (Utilities|FlowControl|Delay 1.0)
      (Utilities|FlowControl|Delay 3.4)
      (|IceSpawn))))

(event EventBeginPlay
  ;[1 1 1] 〇秒ごとに
  (Utilities|Time|SetTimerbyEvent (delegate Custom|Spawn_Ice%201) 1.8 true))

(fn ConstructionScript)